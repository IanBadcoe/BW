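; Player controller that removes the camera manager's view roll restriction and handles yaw camera input relative to the pawn's own up vector.
; On BeginPlay it widens the roll limits to nearly a full circle and caches the player's BP_Pawn.
; The yaw axis input, scaled by frame time and pawn YawScale, becomes an axis-angle rotation fed into roll, pitch and yaw input, ignoring very small values.
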(event EventBeginPlay
  (bind _returnvalue (Game|GetPlayerCameraManager 0))
  (Variables|/Script/Engine.PlayerCameraManager|SetViewRollMax _returnvalue 359.998993)
  (Variables|/Script/Engine.PlayerCameraManager|SetViewRollMin _returnvalue 0.0)
  (|CallParentFunction)
  (bind _asbp_pawn (Utilities|Casting|CastToBP_Pawn (Game|Player|GetPlayerPawn 0)))
  (Variables|Default|SetMyPawn _asbp_pawn))

(event EventTick
  (params (DeltaSeconds :type Float%20%28single-precision%29))
  (|CallParentFunction DeltaSeconds))

(event Input|AxisEvents|InputAxisCameraYawAxis
  (params (AxisValue :type Float%20%28single-precision%29))
  (bind _returnvalue (Utilities|Time|GetWorldDeltaSeconds))
  (bind _mypawn (Variables|Default|GetMyPawn))
  (bind _mypawn_2 (Variables|Default|GetMyPawn))
  (bind _returnvalue_2 (Transformation|GetActorUpVector _mypawn_2))
  (bind _yawscale (Variables|/Game/Blueprints/BP_Pawn.BP_Pawn_C|GetYawScale _mypawn))
  (bind _returnvalue_3 (* AxisValue _returnvalue _yawscale))
  (bind _returnvalue_4 (Math|Vector|RotatorfromAxisandAngle _returnvalue_2 _returnvalue_3))
  (if (> (Math|Float|Absolute(Float) _returnvalue_3) 0.1)
    (Class|PlayerController|AddRollInput (.roll _returnvalue_4))
    (Class|PlayerController|AddPitchInput (.pitch _returnvalue_4))
    (Class|PlayerController|AddYawInput (.yaw _returnvalue_4))))

(fn ConstructionScript)