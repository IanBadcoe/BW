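; BP_Pawn2 is a player-controlled pawn with custom gravity that follows the surface beneath it.
; Each tick it traces along the last gravity direction for WorldStatic geometry, taking the negated hit normal as new gravity or accumulating fall velocity into MovementComponent input on a miss.
; Input axes drive movement along actor forward/right and controller look, with YawScale scaling both yaw and pitch.
; Rotation alignment to the surface is present but unconnected.
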(event EventBeginPlay)

(event Collision|EventActorBeginOverlap
  (params (OtherActor :type Actor%20Object%20Reference)))

(event EventTick
  (params (DeltaSeconds :type Float%20%28single-precision%29))
  (bind _returnvalue (Transformation|GetActorLocation))
  (bind (_outhit _returnvalue_2) (Collision|LineTraceForObjects _returnvalue (+ _returnvalue (* (Variables|Default|GetLastGravity) 1e+02)) (Utilities|Array|MakeArray "ObjectTypeQuery1") false (Utilities|Array|MakeArray self) "None"))
  (if _returnvalue_2
    (Variables|Default|SetLastGravityVelocity "0, 0, 0")
    (Variables|Default|SetLastGravity (Math|Vector|NegateVector (.ImpactNormal (Collision|BreakHitResult _outhit))))
    (else
      (bind _output_get (Variables|Default|SetLastGravityVelocity (+ (* (Variables|Default|GetLastGravity) (* (Variables|Default|GetGravityStrength) (Utilities|Time|GetWorldDeltaSeconds))) (Variables|Default|GetLastGravityVelocity))))
      (Class|PawnMovementComponent|AddInputVector (Variables|Default|GetMovementComponent) (* _output_get (Utilities|Time|GetWorldDeltaSeconds)) false))))

(event Input|AxisEvents|InputAxisFBMoveControlAxis
  (params (AxisValue :type Float%20%28single-precision%29))
  (Class|PawnMovementComponent|AddInputVector (Variables|Default|GetMovementComponent) (* (Transformation|GetActorForwardVector) AxisValue) false))

(event Input|AxisEvents|InputAxisRLMoveControlAxis
  (params (AxisValue :type Float%20%28single-precision%29))
  (Class|PawnMovementComponent|AddInputVector (Variables|Default|GetMovementComponent) (* (Transformation|GetActorRightVector) AxisValue) false))

(event Input|AxisEvents|InputAxisCameraPanAxis
  (params (AxisValue :type Float%20%28single-precision%29))
  (Pawn|Input|AddControllerYawInput (* AxisValue (Utilities|Time|GetWorldDeltaSeconds) (Variables|Default|GetYawScale))))

(event Input|AxisEvents|InputAxisCameraPitchAxis
  (params (AxisValue :type Float%20%28single-precision%29))
  (Pawn|Input|AddControllerPitchInput (* AxisValue (Utilities|Time|GetWorldDeltaSeconds) (Variables|Default|GetYawScale))))

(fn ConstructionScript)