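; Player pawn with surface-relative gravity, letting it move over floors of any orientation.
; Each tick, DetectFloor traces along the last gravity direction; a hit resets fall velocity, points gravity into the surface and realigns control rotation via normal cross products.
; ApplyGravity then accumulates fall velocity and feeds it to the movement component as input.
; Input axes drive actor-relative movement, local yaw and limited camera pitch.
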(event EventBeginPlay)

(event Collision|EventActorBeginOverlap
  (params (OtherActor :type Actor%20Object%20Reference)))

(event EventTick
  (params (DeltaSeconds :type Float%20%28single-precision%29))
  (bind (_outhit _returnvalue) (CallFunction|DetectFloor))
  (if _returnvalue
    (Variables|Default|SetLastGravityVelocity "0, 0, 0")
    (Variables|Default|SetLastGravity (Math|Vector|NegateVector (.ImpactNormal (Collision|BreakHitResult _outhit))))
    (bind _rotation (CallFunction|GetSurfaceRelativeRotation (.ImpactNormal (Collision|BreakHitResult _outhit)) (Pawn|GetControlRotation :!class /Script/Engine.Pawn)))
    (Pawn|SetControlRotation (Pawn|GetController) _rotation)
    (CallFunction|ApplyGravity)
    (else
      (CallFunction|ApplyGravity))))

(event Input|AxisEvents|InputAxisFBMoveControlAxis
  (params (AxisValue :type Float%20%28single-precision%29))
  (Class|PawnMovementComponent|AddInputVector (Variables|Default|GetMovementComponent) (* (Transformation|GetActorForwardVector) AxisValue) false))

(event Input|AxisEvents|InputAxisRLMoveControlAxis
  (params (AxisValue :type Float%20%28single-precision%29))
  (Class|PawnMovementComponent|AddInputVector (Variables|Default|GetMovementComponent) (* (Transformation|GetActorRightVector) AxisValue) false))

(event Input|AxisEvents|InputAxisCameraPanAxis
  (params (AxisValue :type Float%20%28single-precision%29))
  (Transformation|AddActorLocalRotation (Math|Rotator|MakeRotator 0.0 0.0 (* AxisValue (Utilities|Time|GetWorldDeltaSeconds) (Variables|Default|GetYawScale))) false false))

(event Input|AxisEvents|InputAxisCameraPitchAxis
  (params (AxisValue :type Float%20%28single-precision%29))
  (bind _camera (Variables|Default|GetCamera))
  (bind _relativerotation (Variables|/Script/Engine.SceneComponent|GetRelativeRotation _camera))
  (bind _pitch (Math|Rotator|BreakRotator _relativerotation))
  (if (> AxisValue 0.0)
    (if (< _pitch 7e+01)
      (Transformation|AddRelativeRotation (Variables|Default|GetCamera) (Math|Rotator|MakeRotator 0.0 AxisValue 0.0) false false :!label _label))
    (elif (> _pitch -7e+01)
      (goto _label))))

(fn ConstructionScript)

(fn GetSurfaceRelativeRotation
  (params (Normal :type Vector) (CurrentRotation :type Rotator))
  (bind (_x _y _z) (Math|Rotator|BreakRotIntoAxes CurrentRotation))
  (bind _returnvalue (Math|Vector|CrossProduct Normal _x))
  (bind _returnvalue_2 (Math|Vector|CrossProduct _y Normal))
  (bind _returnvalue_3 (Math|Vector|Normalize _returnvalue))
  (bind _returnvalue_4 (Math|Vector|Normalize _returnvalue_2))
  (bind _returnvalue_5 (Math|Rotator|MakeRotationfromAxes _returnvalue_4 _returnvalue_3 Normal))
  (if (Variables|Default|GetLogInputs)
    (Development|PrintString (Utilities|String|BuildString(Vector) (Utilities|String|BuildString(Vector) (Utilities|String|BuildString(Vector) (Utilities|String|BuildString(Vector) "" "N: (" Normal ")") "X: (" _x ")") "Y: (" _y ")") "Z: (" _z ")")))
  (if (Variables|Default|GetLogOutput)
    (Development|PrintString (Utilities|String|ToString(Rotator) _returnvalue_5)))
  (return _returnvalue_5))

(fn DetectFloor
  (bind _returnvalue (Transformation|GetActorLocation))
  (bind (_outhit _returnvalue_2) (Collision|LineTraceForObjects _returnvalue (+ _returnvalue (* (Variables|Default|GetLastGravity) 1e+02)) (Utilities|Array|MakeArray "ObjectTypeQuery1") false (Utilities|Array|MakeArray self) "ForDuration"))
  (return _outhit _returnvalue_2))

(fn ApplyGravity
  (bind _output_get (Variables|Default|SetLastGravityVelocity (+ (* (Variables|Default|GetLastGravity) (* (Variables|Default|GetGravityStrength) (Utilities|Time|GetWorldDeltaSeconds))) (Variables|Default|GetLastGravityVelocity))))
  (Class|PawnMovementComponent|AddInputVector (Variables|Default|GetMovementComponent) (* _output_get (Utilities|Time|GetWorldDeltaSeconds)) false))